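; BP_Fruit is a fruit actor that shatters once when hit.
; Its onHit event, gated by a DoOnce, turns off CollisionMesh collision and swaps the visible FruitMesh for the WatermelonSphereDM destructible.
; It then activates the destructible and applies small-radius damage with an impulse at the Container's location to break it apart.
; Nothing in this graph calls onHit or resets the gate.
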(event `onHit`
  (bind _watermelonsphere_dm (`self.WatermelonSphere_DM`))
  (`/Engine/EditorBlueprintResources/StandardMacros.DoOnce` false
    (:`Completed`
      (`PrimitiveComponent.SetCollisionEnabled` (`self.CollisionMesh`) "NoCollision")
      (`SceneComponent.SetVisibility` (`self.FruitMesh`) false false)
      (`SceneComponent.SetVisibility` _watermelonsphere_dm true false)
      (`ActorComponent.Activate` _watermelonsphere_dm false)
      (`DestructibleComponent.ApplyRadiusDamage` _watermelonsphere_dm 500.0 (`SceneComponent.K2_GetComponentLocation` (`self.Container`)) 10.0 50.0 false))))

(fn `UserConstructionScript`)